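; AI shooter character Blueprint that fires a hitscan weapon at a target enemy.
; On BeginPlay it snaps the gun component to the mesh's hand_r socket.
; ShootEnemy spawns an explosion effect at the gun, then line-traces on Visibility from the character to the target's location.
; Damage applies only when the trace hits that exact target, so blockers prevent damage but there is no aim spread.
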(event `PlayShootEffects`
  (bind _gun (`self.Gun`))
  ;[1 1 1] Gun Effects
  (`GameplayStatics.SpawnEmitterAtLocation` "/Game/StarterContent/Particles/P_Explosion.P_Explosion" (`SceneComponent.GetSocketLocation` _gun "hand_r") (`SceneComponent.GetSocketRotation` _gun "hand_r")))

(event `self.ReceiveBeginPlay`
  ;[1 1 1] Gun Attach
  (`SceneComponent.K2_AttachToComponent` (`self.Gun`) (`self.Mesh`) "hand_r" "SnapToTarget" "SnapToTarget" "SnapToTarget" true))

(event `self.ReceiveActorBeginOverlap`
  (params (OtherActor :type "Actor Object Reference")))

(event `ShootEnemy`
  (params (EnemyToShoot :type "Actor Object Reference"))
  ;[1 1 1] 100% Shoot Enemy
  (`self.PlayShootEffects`)
  (bind (_outhit _returnvalue) (`KismetSystemLibrary.LineTraceSingle` (`self.K2_GetActorLocation`) (`self.K2_GetActorLocation` EnemyToShoot) "TraceTypeQuery1"))
  (if _returnvalue
    (bind (_bblockinghit _binitialoverlap _time _location _impactpoint _normal _impactnormal _physmat _hitactor) (`GameplayStatics.BreakHitResult` _outhit))
    (if (== _hitactor EnemyToShoot)
      (`GameplayStatics.ApplyDamage` _hitactor 10.0 (`self.GetController`) self "/Script/Engine.DamageType"))))

(fn `UserConstructionScript`)