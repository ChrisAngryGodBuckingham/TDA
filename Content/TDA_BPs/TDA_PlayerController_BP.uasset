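; Player controller for the TDA game, handling the in-game menu, inventory screen, mouse look and session exit.
; On BeginPlay it creates the hidden menu widget, loads saved settings, registers with the GameInstance and flags the listen-server player via GameState.
; Escape or the Menu input flip-flops the menu with input mode and cursor; closing reloads settings and removes leftover credits and browser widgets.
; Look axes set control rotation directly using sensitivity and invert options.
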(event `self.ReceiveBeginPlay`
  ;[0.15 0.1327 0.02994] Event Begin Play
  (`self.Create InGameMenu Widget`)
  (`self.Load Game Settings`)
  (`self.Detect Server Type`)
  (`self.Hide Mouse`)
  (`self.Tell GameInstance The Player Controller`))

(event `Key|Escape`
  (params (Key :type "Key Structure" :default "AnyKey"))
  (bind _returnvalue (`GameplayStatics.GetPlayerController` 0))
  (bind _tda_ingamemenu (`self.TDA_InGameMenu`))
  (bind _keybindwidget (`/Game/TDA_Menu/MainMenu/Blueprints/UI/Submenus/TDA_SettingsSubMenu.KeyBindWidget` (`/Game/TDA_Menu/MainMenu/Blueprints/UI/TDA_InGameMenu.TDA_SettingsSubMenu` (`self.TDA_InGameMenu`))))
  ;[0.08001 1 0.05586] Open/close the In Game Menu
  (:`Pressed`
    ;;[1 1 0] We avoid to close In Game Menu on rebind open/close menu key. Not the best solution but it works.
    (if (`/Game/Menus/MainMenu/Blueprints/UI/SettingsPanels/ControlsSettingsDetails.IsMenuKeyBindPressed` _keybindwidget) :!label _label
      (set `/Game/Menus/MainMenu/Blueprints/UI/SettingsPanels/ControlsSettingsDetails.IsMenuKeyBindPressed` false _keybindwidget)
      (else
        (`/Engine/EditorBlueprintResources/StandardMacros.FlipFlop`
          (:`A`
            (`Widget.SetVisibility` _tda_ingamemenu "Visible")
            (`WidgetBlueprintLibrary.SetInputMode_GameAndUIEx` _returnvalue null "LockAlways" false)
            (set `PlayerController.bShowMouseCursor` true _returnvalue)
            (`self.SetIgnoreLookInput` _returnvalue true)
            (`VirtualCursorFunctionLibrary.EnableVirtualCursor` _returnvalue))
          (:`B`
            (`Widget.SetVisibility` _tda_ingamemenu "Collapsed")
            (`WidgetBlueprintLibrary.SetInputMode_GameOnly` _returnvalue)
            (set `PlayerController.bShowMouseCursor` false _returnvalue)
            (`VirtualCursorFunctionLibrary.DisableVirtualCursor` _returnvalue)
            (`self.SetIgnoreLookInput` _returnvalue false)
            ;;[1 0.9952 0.3837] Refresh Game Settings From Save On Menu Close
            (`self.Load Game Settings`)
            ;[1 0.2891 0.8927] Remove About Widgets If Open
            (`|ExecutionSequence`
              (:`then_0`
                (bind _foundwidgets (`WidgetBlueprintLibrary.GetAllWidgetsOfClass` "/Game/TDA_Menu/MainMenu/Blueprints/UI/AboutPanels/TDA_Credits.TDA_Credits_C"))
                (for _array_element _foundwidgets
                  (`Widget.RemoveFromParent` _array_element)))
              (:`then_1`
                (bind _foundwidgets_2 (`WidgetBlueprintLibrary.GetAllWidgetsOfClass` "/Game/TDA_Menu/MainMenu/Blueprints/UI/AboutPanels/TDA_CreditsContainer.TDA_CreditsContainer_C"))
                (for _array_element_2 _foundwidgets_2
                  (`Widget.RemoveFromParent` _array_element_2)))
              (:`then_2`
                (bind _foundwidgets_3 (`WidgetBlueprintLibrary.GetAllWidgetsOfClass` "/Game/TDA_Menu/MainMenu/Blueprints/UI/AboutPanels/TDA_CreditsNavigation.TDA_CreditsNavigation_C"))
                (for _array_element_3 _foundwidgets_3
                  (`Widget.RemoveFromParent` _array_element_3)))
              (:`then_3`
                (`|ExecutionSequence`
                  (:`then_0`
                    (bind _foundwidgets_4 (`WidgetBlueprintLibrary.GetAllWidgetsOfClass` "/Game/TDA_Menu/MainMenu/Blueprints/UI/AboutPanels/TDA_WebBrowser.TDA_WebBrowser_C"))
                    (for _array_element_4 _foundwidgets_4
                      (`Widget.RemoveFromParent` _array_element_4)))
                  (:`then_1`
                    (bind _foundwidgets_5 (`WidgetBlueprintLibrary.GetAllWidgetsOfClass` "/Game/TDA_Menu/MainMenu/Blueprints/UI/AboutPanels/TDA_WebBrowserNavigation.TDA_WebBrowserNavigation_C"))
                    (for _array_element_5 _foundwidgets_5
                      (`Widget.RemoveFromParent` _array_element_5)))
                  (:`then_2`
                    (bind _foundwidgets_6 (`WidgetBlueprintLibrary.GetAllWidgetsOfClass` "/Game/TDA_Menu/MainMenu/Blueprints/UI/AboutPanels/TDA_WebBrowserBackground.TDA_WebBrowserBackground_C"))
                    (for _array_element_6 _foundwidgets_6
                      (`Widget.RemoveFromParent` _array_element_6)))
                  (:`then_3`
                    (bind _foundwidgets_7 (`WidgetBlueprintLibrary.GetAllWidgetsOfClass` "/Game/TDA_Menu/MainMenu/Blueprints/UI/AboutPanels/TDA_WebBrowserContainer.TDA_WebBrowserContainer_C"))
                    (for _array_element_7 _foundwidgets_7
                      (`Widget.RemoveFromParent` _array_element_7))))))))))))

(event `self.ReloadInventory`
  (bind _inventorywidget (`self.InventoryWidget`))
  ;[0.19 0.1691 0.01425] Inventory Functions
  ;;[0.07832 1 0.146] reload inventory after crafting items
  (`/Engine/EditorBlueprintResources/StandardMacros.IsValid` _inventorywidget
    (:`Is Valid`
      (`/Game/UI/Inventory/WB_Inventory.LoadInventoryItems` (cast `/Game/UI/Inventory/WB_Inventory` _inventorywidget :!pure true)))))

(event `InputAction|Menu`
  (params (Key :type "Key Structure" :default "AnyKey"))
  ;[0.08001 1 0.05586] Open/close the In Game Menu
  (:`Pressed`
    (goto _label)))

(event `Create InGameMenu Widget`
  ;[1 0.2891 0.8927] Creates InGameMenu widget
  (bind _returnvalue (`|CreateWidget` "/Game/TDA_Menu/MainMenu/Blueprints/UI/TDA_InGameMenu.TDA_InGameMenu_C"))
  (bind _output_get (set `self.TDA_InGameMenu` _returnvalue))
  (`UserWidget.AddToViewport` _output_get 5)
  (`Widget.SetVisibility` _output_get "Collapsed")
  (set `/Game/TDA_Menu/MainMenu/Blueprints/UI/TDA_InGameMenu.OwningPlayerController` self _returnvalue)
  (`KismetSystemLibrary.Delay` 2.0)
  (set `/Game/TDA_Menu/MainMenu/Blueprints/UI/TDA_InGameMenu.IsListenServer?` (`self.IsListenServer`) _returnvalue)
  (`self.Load Game Settings`))

(event `InputAction|OpenInventory`
  (params (Key :type "Key Structure" :default "AnyKey"))
  (bind _returnvalue (`GameplayStatics.GetPlayerController` 0))
  ;[0.19 0.1691 0.01425] Inventory Functions
  ;;[0.2314 1 0.1848] Open Inventory Screen via I key
  (:`Pressed`
    (`/Engine/EditorBlueprintResources/StandardMacros.IsValid` (`self.InventoryWidget`)
      (:`Is Valid`
        _)
      (:`Is Not Valid`
        (bind _returnvalue_2 (`|CreateWidget` "/Game/UI/Inventory/WB_Inventory.WB_Inventory_C" _returnvalue))
        (bind _output_get (set `self.InventoryWidget` _returnvalue_2))))
    (`UserWidget.AddToViewport` _output_get 0)
    (`WidgetBlueprintLibrary.SetInputMode_UIOnlyEx` _returnvalue (`self.InventoryWidget`))
    (set `self.bShowMouseCursor` true)))

(event `Load Game Settings`
  ;[1 0.9952 0.3837] Load Game Settings On Controller Creation
  (bind _returnvalue (`GameplayStatics.LoadGameFromSlot` "GameSettings"))
  (bind _astda_bp_game_settings_save (cast `/Game/TDA_Menu/MainMenu/Blueprints/Saves/TDA_BP_GameSettingsSave` _returnvalue))
  (set `/Game/TDA_Menu/MainMenu/Blueprints/Saves/TDA_BP_GameSettingsSave.MouseSensitivity` (`/Game/TDA_Menu/MainMenu/Blueprints/Saves/TDA_BP_GameSettingsSave.MouseSensitivity` _astda_bp_game_settings_save) _astda_bp_game_settings_save)
  (set `/Game/TDA_Menu/MainMenu/Blueprints/Saves/TDA_BP_GameSettingsSave.InvertYAxis` (`/Game/TDA_Menu/MainMenu/Blueprints/Saves/TDA_BP_GameSettingsSave.InvertYAxis` _astda_bp_game_settings_save) _astda_bp_game_settings_save)
  (set `/Game/TDA_Menu/MainMenu/Blueprints/Saves/TDA_BP_GameSettingsSave.InvertXAxis` (`/Game/TDA_Menu/MainMenu/Blueprints/Saves/TDA_BP_GameSettingsSave.InvertXAxis` _astda_bp_game_settings_save) _astda_bp_game_settings_save)
  (set `/Game/TDA_Menu/MainMenu/Blueprints/Saves/TDA_BP_GameSettingsSave.PlayerFOV` (`/Game/TDA_Menu/MainMenu/Blueprints/Saves/TDA_BP_GameSettingsSave.PlayerFOV` _astda_bp_game_settings_save) _astda_bp_game_settings_save)
  (bind _astda_character_bp (cast `/Game/BluePrints/TDA_BPs/TDA_Character_BP` (`self.K2_GetPawn`))
    (:`then`
      (`CameraComponent.SetFieldOfView` (`TheDaysAfterCharacter.FollowCamera` _astda_character_bp) (`self.PlayerFOV`)))
    (:`CastFailed`
      ;;[1 0.02 0.02] Debugg
      (`KismetSystemLibrary.PrintString` "Cast failed at loadgamesettings Playercontroller_BP"))))

(event `InputAxis|LookDown`
  (params (AxisValue :type "Float (single-precision)"))
  ;[1 1 1] Set Control Rotation
  (if (`self.InvertYAxis`)
    (set `self.YAxisInput` AxisValue)
    (else
      (set `self.YAxisInput` (* AxisValue -1.0))))
  (`self.SetControlRotation` (`KismetMathLibrary.MakeRotator` (.roll (`self.GetControlRotation`)) (+ (* (* (`self.YAxisInput`) (`self.MouseSensitivity`)) 5.0) (.pitch (`self.GetControlRotation`))) (.yaw (`self.GetControlRotation`))) :!label _label_2))

(event `InputAxis|LookUp`
  (params (AxisValue :type "Float (single-precision)"))
  ;[1 1 1] Set Control Rotation
  (if (`self.InvertYAxis`)
    (set `self.YAxisInput` AxisValue)
    (goto _label_2)
    (else
      (set `self.YAxisInput` (* AxisValue -1.0))
      (goto _label_2))))

(event `Detect Server Type`
  (bind _printdebugonscreen (`self.PrintDebugOnScreen`))
  (bind _printdebugonscreen_2 (`self.PrintDebugOnScreen`))
  ;[0.312 0.3018 0.57] Detects if Dedicated Server or Listen Server - Marks Listen Server Player
  (`KismetSystemLibrary.Delay` 1.0)
  (`/Engine/EditorBlueprintResources/ActorMacros.Switch Has Authority`
    (:`Authority`
      (if (`KismetSystemLibrary.IsDedicatedServer`)
        (`KismetSystemLibrary.PrintString` "A Dedicated Server Is Running The Game" _printdebugonscreen _printdebugonscreen)
        (else
          (`|ExecutionSequence`
            (:`then_0`
              (bind _astda_game_state (cast `/Game/BluePrints/TDA_BPs/TDA_GameState` (`GameplayStatics.GetGameState`)))
              (if (not (`/Game/BluePrints/TDA_BPs/TDA_GameState.IsListenServerAlreadyJoined?` _astda_game_state))
                (set `self.IsListenServer` true)
                (`KismetSystemLibrary.PrintString` "A Listen Server Is Running The Game" _printdebugonscreen_2 _printdebugonscreen_2)))
            (:`then_1`
              (bind _astda_game_state_2 (cast `/Game/BluePrints/TDA_BPs/TDA_GameState` (`GameplayStatics.GetGameState`)))
              (`/Game/BluePrints/TDA_BPs/TDA_GameState.Player Join` _astda_game_state_2))))))))

(event `Hide Mouse`
  (bind _returnvalue (`GameplayStatics.GetPlayerController` 0))
  ;[0.37 0.0074 0.0074] Hide Mouse
  (`WidgetBlueprintLibrary.SetInputMode_GameOnly` _returnvalue)
  (set `PlayerController.bShowMouseCursor` false _returnvalue))

(event `InputAxis|TurnLeft`
  (params (AxisValue :type "Float (single-precision)"))
  ;[1 1 1] Set Control Rotation
  (if (`self.InvertXAxis`)
    (set `self.XAxisInput` (* AxisValue -1.0))
    (else
      (set `self.XAxisInput` AxisValue)))
  (`self.SetControlRotation` (`KismetMathLibrary.MakeRotator` (.roll (`self.GetControlRotation`)) (.pitch (`self.GetControlRotation`)) (+ (* (* (`self.XAxisInput`) (`self.MouseSensitivity`)) 5.0) (.yaw (`self.GetControlRotation`)))) :!label _label_3))

(event `InputAxis|TurnRight`
  (params (AxisValue :type "Float (single-precision)"))
  ;[1 1 1] Set Control Rotation
  (if (`self.InvertXAxis`)
    (set `self.XAxisInput` (* AxisValue -1.0))
    (goto _label_3)
    (else
      (set `self.XAxisInput` AxisValue)
      (goto _label_3))))

(event `Tell GameInstance The Player Controller`
  ;[0.38 0.3361 0.07585] Tell GameInstance The Player Controller
  (bind _asbp_game_instance (cast `/Game/Menus/MainMenu/Blueprints/BP_GameInstance` (`GameplayStatics.GetGameInstance`)))
  (set `/Game/Menus/MainMenu/Blueprints/BP_GameInstance.PlayerController` self _asbp_game_instance))

(event `End Client Online Session`
  (bind _printdebugonscreen (`self.PrintDebugOnScreen`))
  ;[0.312 0.3018 0.57] Client End Online Session
  (`DestroySessionCallbackProxy.DestroySession` self
    (:`then`
      (`KismetSystemLibrary.Delay` 1.0)
      (`GameplayStatics.OpenLevel` "TDA_MainMenu"))
    (:`OnSuccess`
      (`KismetSystemLibrary.PrintString` "Client Destroy Session Success" _printdebugonscreen _printdebugonscreen))))

(fn `UserConstructionScript`)