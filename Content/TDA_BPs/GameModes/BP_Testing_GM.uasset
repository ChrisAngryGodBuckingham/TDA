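; BP_Testing_GM is a testing game mode that controls background music and the security alarm sound.
; It starts its AudioMusic component on BeginPlay.
; The SecurityAlarmInterface event takes a SendAlarm flag, sets the sound on that same component in either branch, and restarts playback from the beginning.
; SceneCaptureActivation is an empty stub, as is the construction script.
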(event `self.ReceiveBeginPlay`
  ;[0.312 0.3018 0.57] Music Set Up
  (`AudioComponent.Play` (`self.Audio_music`) 0.0))

(event `/Game/BluePrints/AllLevels/SecurityCameras/BPI_AlarmIntrface.SecurityAlarmInterface`
  (params (SendAlarm :type Boolean))
  (bind _audio_music (`self.Audio_music`))
  ;[0.0861 0.5189 0.57] Interface Event that enables/disables Alarm Sound
  (if SendAlarm
    (`AudioComponent.SetSound` _audio_music null)
    (`AudioComponent.Play` _audio_music 0.0)
    (else
      (`AudioComponent.SetSound` _audio_music null)
      (`AudioComponent.Play` _audio_music 0.0))))

(fn `SceneCaptureActivation`
  (params (Activation :type Boolean))
  (returns (CaptureTexture :type "TextureRenderTarget2D Object Reference"))
  (return null))

(fn `UserConstructionScript`)