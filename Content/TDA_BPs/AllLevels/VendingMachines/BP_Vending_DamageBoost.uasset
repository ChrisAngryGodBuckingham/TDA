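; A damage boost vending machine that sells player damage upgrades for points.
; Its trigger overlap stores the TDA_Onslaught_Character and shows the buy text, and leaving hides the text without clearing that reference.
; UseEvent checks Points against BoosterCost, then deducts it, raises PlayerDamage by a small fixed step plus BoostAmount and plays the buy sound, or plays an error sound.
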(event `self.BuyTrigger.OnComponentBeginOverlap`
  (params (OverlappedComponent :type "PrimitiveComponent Object Reference") (OtherActor :type "Actor Object Reference") (OtherComp :type "PrimitiveComponent Object Reference") (OtherBodyIndex :type Integer) (bFromSweep :type Boolean) (SweepResult :type "HitResult Structure (by ref)"))
  (bind _astda_onslaught_character (cast `/Game/BluePrints/GameModes/GM_Onslaught/TDA_Onslaught_Character` OtherActor))
  (`SceneComponent.SetVisibility` (`self.BuyText`) true false))

(event `InputAction|Use`
  (params (Key :type "Key Structure" :default "AnyKey"))
  (bind _boostercost (`self.BoosterCost`))
  (:`Pressed`
    (bind _points (`/Game/BluePrints/GameModes/GM_Onslaught/TDA_Onslaught_Character.Points` (stale `self.BuyTrigger.OnComponentBeginOverlap` _astda_onslaught_character)))
    (if (>= _points _boostercost)
      (set `/Game/BluePrints/GameModes/GM_Onslaught/TDA_Onslaught_Character.Points` (- _points _boostercost) (stale `self.BuyTrigger.OnComponentBeginOverlap` _astda_onslaught_character))
      (set `/Game/BluePrints/GameModes/GM_Onslaught/TDA_Onslaught_Character.PlayerDamage` (+ (`/Game/BluePrints/GameModes/GM_Onslaught/TDA_Onslaught_Character.PlayerDamage` (stale `self.BuyTrigger.OnComponentBeginOverlap` _astda_onslaught_character)) 0.01) (stale `self.BuyTrigger.OnComponentBeginOverlap` _astda_onslaught_character))
      (`|ExecutionSequence`
        (:`then_0`
          (`/Game/BluePrints/GameModes/GM_Onslaught/TDA_Onslaught_Character.BuySound` (stale `self.BuyTrigger.OnComponentBeginOverlap` _astda_onslaught_character)))
        (:`then_1`
          (set `/Game/BluePrints/GameModes/GM_Onslaught/TDA_Onslaught_Character.PlayerDamage` (+ (`/Game/BluePrints/GameModes/GM_Onslaught/TDA_Onslaught_Character.PlayerDamage` (stale `self.BuyTrigger.OnComponentBeginOverlap` _astda_onslaught_character)) (`self.BoostAmount`)) (stale `self.BuyTrigger.OnComponentBeginOverlap` _astda_onslaught_character))))
      (else
        (`/Game/BluePrints/GameModes/GM_Onslaught/TDA_Onslaught_Character.ErrorSound` (stale `self.BuyTrigger.OnComponentBeginOverlap` _astda_onslaught_character))))))

(event `self.BuyTrigger.OnComponentEndOverlap`
  (params (OverlappedComponent :type "PrimitiveComponent Object Reference") (OtherActor :type "Actor Object Reference") (OtherComp :type "PrimitiveComponent Object Reference") (OtherBodyIndex :type Integer))
  (cast `/Game/BluePrints/GameModes/GM_Onslaught/TDA_Onslaught_Character` OtherActor)
  (`SceneComponent.SetVisibility` (`self.BuyText`) false false))

(fn `UserConstructionScript`)