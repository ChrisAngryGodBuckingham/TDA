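; BP_Security_Flashing_Lights is an alarm beacon that switches between an off light and a rotating spot light when it receives a security alarm interface call.
; The alarm state toggles both lights' visibility, sets a scalar on the mesh's dynamic material and opens or closes a gate on Tick.
; While open, the gate spins the spot light's yaw, scaled by delta time.
; Construction applies the on/off colours and creates the material instance.
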(event `self.ReceiveTick`
  (params (DeltaSeconds :type "Float (single-precision)"))
  (bind _spotlight (`self.SpotLight`))
  ;[1 1 1] Spot Light Rotation
  (`/Engine/EditorBlueprintResources/StandardMacros.Gate` true :!label _label
    (:`Exit`
      (`SceneComponent.K2_SetRelativeRotation` _spotlight (`KismetMathLibrary.MakeRotator` (.roll (`SceneComponent.RelativeRotation` _spotlight)) (.pitch (`SceneComponent.RelativeRotation` _spotlight)) (+ (.yaw (`SceneComponent.RelativeRotation` _spotlight)) (* (`self.LightRotationSpeed`) DeltaSeconds))) false false))))

(event `/Game/BluePrints/AllLevels/SecurityCameras/BPI_AlarmIntrface.SecurityAlarmInterface`
  (params (SendAlarm :type Boolean))
  (bind _alarmstate (`self.AlarmState`))
  (bind _alarmstate_2 (`self.AlarmState`))
  (set `self.AlarmState` SendAlarm)
  (if SendAlarm
    ;[1 1 1] Alarm on Settings
    (`SceneComponent.SetVisibility` (`self.SpotLight`) _alarmstate_2 false)
    (`SceneComponent.SetVisibility` (`self.OffLight`) (not _alarmstate_2) false)
    (`MaterialInstanceDynamic.SetScalarParameterValue` (`self.AlarmMaterial`) "AlarmState" 1.0) ; Turn ON alpha from material
    (goto _label :!via `Open`)
    (else
      ;[1 1 1] Alarm off settings
      (`SceneComponent.SetVisibility` (`self.SpotLight`) _alarmstate false)
      (`SceneComponent.SetVisibility` (`self.OffLight`) (not _alarmstate) false)
      (`MaterialInstanceDynamic.SetScalarParameterValue` (`self.AlarmMaterial`) "AlarmState" 0.0) ; Turn OFF Material through Alpha->AlarmState material property
      (goto _label :!via `Close`))))

(fn `SceneCaptureActivation`
  (params (Activation :type Boolean))
  (returns (CaptureTexture :type "TextureRenderTarget2D Object Reference"))
  (return null))

(fn `UserConstructionScript`
  ;[1 1 1] Set Light Colours
  (`LightComponent.SetLightColor` (`self.OffLight`) (`self.AlarmOffColour`) true)
  (`LightComponent.SetLightColor` (`self.SpotLight`) (`self.AlarmOnColour`) true)
  ;[1 1 1] Create Dynamic Material
  (bind _returnvalue (`PrimitiveComponent.CreateDynamicMaterialInstance` (`self.LightMesh`) 0 null))
  (set `self.AlarmMaterial` _returnvalue))