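; Security monitor actor that cycles its screen through the feeds of a list of camera Blueprints.
; Construction configures screen audio and creates a dynamic screen material.
; MonitorCameraSwap switches off the previous camera's scene capture, advances with wraparound, then applies the texture returned by activating the next camera, plus its label.
; A timeline animates material noise during each swap, and only the selected camera is left capturing.
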(event `/Game/BluePrints/AllLevels/SecurityCameras/BPI_AlarmIntrface.MonitorCameraSwap`
  (bind _monitormaterial (`self.MonitorMaterial`))
  (bind _cameraindex (`self.CameraIndex`))
  (message `/Game/BluePrints/AllLevels/SecurityCameras/BPI_AlarmIntrface.SceneCaptureActivation` (`|GetArrayItem` (`self.CameraBPs`) (`self.PreviousIndex`)) false)
  (`|ExecutionSequence`
    (:`then_0`
      (bind (_direction _noiseanim) (`Timeline|ScreenNoiseAnim` :!via `PlayFromStart`)
        (:`Update`
          (`MaterialInstanceDynamic.SetScalarParameterValue` (`self.MonitorMaterial`) "Noise" _noiseanim))))
    (:`then_1`
      (if (< (`self.CameraIndex`) (- (`KismetArrayLibrary.Array_Length` (`self.CameraBPs`)) 1))
        (set `self.CameraIndex` (+ (`self.CameraIndex`) 1))
        (else
          (set `self.CameraIndex` 0)))
      (bind _capturetexture (message `/Game/BluePrints/AllLevels/SecurityCameras/BPI_AlarmIntrface.SceneCaptureActivation` (`|GetArrayItem` (`self.CameraBPs`) (`self.CameraIndex`)) true))
      (`MaterialInstanceDynamic.SetTextureParameterValue` _monitormaterial "ScreenTexture" _capturetexture)
      (`MaterialInstanceDynamic.SetScalarParameterValue` _monitormaterial "CameraLabel" (`KismetMathLibrary.Conv_IntToDouble` _cameraindex))
      (set `self.PreviousIndex` _cameraindex))))

(fn `SceneCaptureActivation`
  (params (Activation :type Boolean))
  (returns (CaptureTexture :type "TextureRenderTarget2D Object Reference"))
  (return null))

(fn `UserConstructionScript`
  (bind _audio_screen (`self.Audio_Screen`))
  ;[1 1 1] Audio Components
  (`AudioComponent.SetVolumeMultiplier` _audio_screen (`self.SetVolume`))
  (`AudioComponent.SetPitchMultiplier` _audio_screen (`self.SetPitch`))
  (`AudioComponent.SetSound` (`self.Audio_Screen`) (`self.ScreenSoundCue`))
  ;[1 1 1] Visual components
  (bind _returnvalue (`PrimitiveComponent.CreateDynamicMaterialInstance` (`self.MonitorMesh`) 1 "/Game/BluePrints/AllLevels/SecurityCameras/Materials/M_SecurityCamera_Screen.M_SecurityCamera_Screen"))
  (set `self.MonitorMaterial` _returnvalue))