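; Security sliding double door that toggles between its open and closed states on alarm pulses received through SecurityAlarmInterface.
; Each true pulse checks the Open flag, plays a door sound and runs one of two timelines; a false signal only clears AlarmOn.
; The timelines lerp both leaves between their start positions and mirrored DoorOpenOffset locations.
; The construction script applies each leaf's configurable start position and scale.
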(event `/Game/BluePrints/AllLevels/SecurityCameras/BPI_AlarmIntrface.SecurityAlarmInterface`
  (params (SendAlarm :type Boolean))
  ;[1 1 1] Listen for Alarm Pulse
  (if SendAlarm :!label _label
    (set `self.AlarmOn` true)
    (else
      (set `self.AlarmOn` false)))
  (if (`self.AlarmOn`)
    ;[0.0861 0.5189 0.57] Check open state of doors
    (if (`self.Open?`)
      ;[0.0093 0.31 0.03664 0.781] Audio and Animations
      (`GameplayStatics.PlaySoundAtLocation` "/Game/BluePrints/AllLevels/SecurityCameras/Audio/Blueprints_DoorOpen01_Cue.Blueprints_DoorOpen01_Cue" (`self.K2_GetActorLocation`))
      (bind (_direction _closedooranim) (`Timeline|CloseAnim` :!via `PlayFromStart`) ; Door Close Animation
        (:`Update`
          _)
        (:`Finished`
          _))
      ;[0.37 0.0074 0.0074] Closed State
      (set `self.Open?` false)
      (`SceneComponent.K2_SetRelativeLocation` (`self.LeftDoor`) (`KismetMathLibrary.VLerp` (`self.LeftDoorStart`) (* (`self.DoorOpenOffset`) -1) _closedooranim) false false)
      (`SceneComponent.K2_SetRelativeLocation` (`self.RightDoor`) (`KismetMathLibrary.VLerp` (`self.RightDoorStart`) (`self.DoorOpenOffset`) _closedooranim) false false)
      (else
        (`GameplayStatics.PlaySoundAtLocation` "/Game/BluePrints/AllLevels/SecurityCameras/Audio/Blueprints_DoorClose01_Cue.Blueprints_DoorClose01_Cue" (`self.K2_GetActorLocation`))
        (bind (_direction_2 _dooropenanimation) (`Timeline|OpenDoorAnim`)
          (:`Update`
            _)
          (:`Finished`
            _))
        ;[0.156 1 0.2327] Open State
        (set `self.Open?` true)
        (`SceneComponent.K2_SetRelativeLocation` (`self.LeftDoor`) (`KismetMathLibrary.VLerp` (* (`self.DoorOpenOffset`) -1) (`self.LeftDoorStart`) _dooropenanimation) false false)
        (`SceneComponent.K2_SetRelativeLocation` (`self.RightDoor`) (`KismetMathLibrary.VLerp` (`self.DoorOpenOffset`) (`self.RightDoorStart`) _dooropenanimation) false false)))))

(event `self.ReceiveBeginPlay`
  ;[1 1 1] Listen for Alarm Pulse
  (goto _label))

(fn `SceneCaptureActivation`
  (params (Activation :type Boolean))
  (returns (CaptureTexture :type "TextureRenderTarget2D Object Reference"))
  (return null))

(fn `UserConstructionScript`
  ;[1 1 1] Left Door
  (`SceneComponent.K2_SetRelativeLocation` (`self.LeftDoor`) (`self.LeftDoorStart`) false false)
  (`SceneComponent.SetRelativeScale3D` (`self.LeftDoor`) (`self.LeftDoorSize`))
  ;[1 1 1] Right Door
  (`SceneComponent.K2_SetRelativeLocation` (`self.RightDoor`) (`self.RightDoorStart`) false false)
  (`SceneComponent.SetRelativeScale3D` (`self.RightDoor`) (`self.RightDoorSize`)))