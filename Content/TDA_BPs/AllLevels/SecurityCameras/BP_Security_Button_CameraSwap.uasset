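; Interactive security-room button that tells linked screen Blueprints to swap their monitor camera.
; Overlapping the trigger enables input and spawns prompt text at an arrow, rotated toward the player camera on Tick and destroyed on exit.
; While overlapped, E or Use plays a click, sends the swap message through ScreenBPs and animates the press with a timeline.
; The construction script applies volume and pitch to control-room and interior audio.
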(event `self.ButtonTrigger.OnComponentBeginOverlap`
  (params (OverlappedComponent :type "PrimitiveComponent Object Reference") (OtherActor :type "Actor Object Reference") (OtherComp :type "PrimitiveComponent Object Reference") (OtherBodyIndex :type Integer) (bFromSweep :type Boolean) (SweepResult :type "HitResult Structure (by ref)"))
  (bind _textcomponent (`self.TextComponent`))
  ;[1 0.993 0.095] Add / Remove Trigger text during overlap
  (`|ExecutionSequence`
    (:`then_0`
      (if true
        (set `self.ButtonCollisionTrigger` true)
        (`self.EnableInput` (`GameplayStatics.GetPlayerController` 0))))
    (:`then_1`
      (bind _returnvalue (`AddComponent|NODE_AddTextRenderComponent-0`))
      (`SceneComponent.SetVisibility` _returnvalue false false)
      (set `self.TextComponent` _returnvalue)
      ;[0.156 1 0.2327] Draw text and align to player view
      (if (`KismetSystemLibrary.IsValid` _textcomponent) :!label _label
        (`SceneComponent.K2_SetWorldLocation` _textcomponent (`SceneComponent.K2_GetComponentLocation` (`self.TextArrow`)) false false)
        (`SceneComponent.K2_SetWorldRotation` _textcomponent (`KismetMathLibrary.MakeRotFromX` (- (`self.K2_GetActorLocation` (`GameplayStatics.GetPlayerCameraManager` 0)) (`SceneComponent.K2_GetComponentLocation` (`self.TextArrow`)))) false false)
        (`SceneComponent.SetVisibility` (`self.TextComponent`) true false)))))

(event `self.ReceiveTick`
  (params (DeltaSeconds :type "Float (single-precision)"))
  ;[0.156 1 0.2327] Draw text and align to player view
  (goto _label))

(event `self.ButtonTrigger.OnComponentEndOverlap`
  (params (OverlappedComponent :type "PrimitiveComponent Object Reference") (OtherActor :type "Actor Object Reference") (OtherComp :type "PrimitiveComponent Object Reference") (OtherBodyIndex :type Integer))
  (bind _textcomponent (`self.TextComponent`))
  ;[1 0.993 0.095] Add / Remove Trigger text during overlap
  (`|ExecutionSequence`
    (:`then_0`
      (if true
        (set `self.ButtonCollisionTrigger` false)))
    (:`then_1`
      (if (`KismetSystemLibrary.IsValid` _textcomponent)
        (`ActorComponent.K2_DestroyComponent` _textcomponent)))))

(event `Key|E`
  (params (Key :type "Key Structure" :default "AnyKey"))
  (bind _screenbps (`self.ScreenBPs`))
  ;[1 0.2891 0.8927] Interaction Key
  (:`Pressed`
    (if (`self.ButtonCollisionTrigger`) :!label _label_2
      ;[1 1 1] Button Audio
      (`GameplayStatics.PlaySoundAtLocation` "/Game/BluePrints/AllLevels/SecurityCameras/Audio/Blueprints_ButtonPush01.Blueprints_ButtonPush01" (`SceneComponent.K2_GetComponentLocation` (`self.Button`)) (struct) 0.2) ; ButtonPressed Sound
      ;[1 0.993 0.095] Transmits Key press to Interface
      (for _index (range (`KismetArrayLibrary.Array_Length` _screenbps))
        (message `/Game/BluePrints/AllLevels/SecurityCameras/BPI_AlarmIntrface.MonitorCameraSwap` (`|GetArrayItem` _screenbps _index))
        (bind (_direction _press) (`Timeline|ButtonPress` :!via `PlayFromStart`)
          (:`Update`
            (`SceneComponent.K2_SetRelativeLocation` (`self.Button`) (`KismetMathLibrary.MakeVector` 0.0 0.0 _press) false false)))))))

(event `InputAction|Use`
  (params (Key :type "Key Structure" :default "AnyKey"))
  ;[1 0.2891 0.8927] Interaction Key
  (:`Pressed`
    (goto _label_2)))

(fn `SceneCaptureActivation`
  (params (Activation :type Boolean))
  (returns (CaptureTexture :type "TextureRenderTarget2D Object Reference"))
  (return null))

(fn `UserConstructionScript`
  (bind _controlroomaudio (`self.ControlRoomAudio`))
  (bind _interioraudio (`self.InteriorAudio`))
  (`AudioComponent.SetVolumeMultiplier` _controlroomaudio (`self.ControlRoomVolume`))
  (`AudioComponent.SetPitchMultiplier` _controlroomaudio (`self.ControlRoomPitch`))
  (`AudioComponent.SetVolumeMultiplier` _interioraudio (`self.InteriorVolume`))
  (`AudioComponent.SetPitchMultiplier` _interioraudio (`self.InteriorPitch`)))