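; Security camera that sweeps on a timeline until the player enters its view cone, then tracks the pawn within clamped pitch and yaw.
; Detection switches light colour and audio, and notifies linked Blueprints, plus optionally the GameMode for music, through an alarm interface.
; Leaving the view capsule starts a delay timeline that clears the alarm unless re-entry stops it.
; Construction configures light, dynamic materials and a render-target scene capture with toggleable visibility.
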(event `self.SM_Security_Camera_Viewcone.OnComponentBeginOverlap`
  (params (OverlappedComponent :type "PrimitiveComponent Object Reference") (OtherActor :type "Actor Object Reference") (OtherComp :type "PrimitiveComponent Object Reference") (OtherBodyIndex :type Integer) (bFromSweep :type Boolean) (SweepResult :type "HitResult Structure (by ref)"))
  (bind _audioscanner (`self.AudioScanner`))
  (bind _audioscanner_2 (`self.AudioScanner`))
  (bind _bptotriggeralarm (`self.BPToTriggerAlarm`))
  (bind _hastarget (`self.HasTarget`))
  (bind _returnvalue (`SceneComponent.K2_GetComponentLocation` (`self.SM_CCTVCamera`)))
  ;[1 0.993 0.095] Alarm States and Materials + Light colours
  (if (`self.HasTarget`)
    (`Timeline|AlarmDelay` :!via `Stop` :!label _label
      (:`Finished`
        (set `self.HasTarget` false)
        ;;[1 0.9952 0.3837] Audio Components
        (`GameplayStatics.PlaySoundAtLocation` "/Game/BluePrints/TDA_BPs/Interactive_Objects/SecurityCameras/Assets/Audio/Assets/Audio/Blueprint_Music_Stealth02.Blueprint_Music_Stealth02" _returnvalue)
        (`AudioComponent.SetSound` _audioscanner_2 (`self.ScanResetCue`))
        (`ActorComponent.Activate` _audioscanner_2 false) ; Play Audio
        (`LightComponent.SetLightColor` (`self.SpotLight`) (`self.LightColourAlarmOff`) true) ; Alarm OFF
        (`MaterialInstanceDynamic.SetScalarParameterValue` (`self.ViewConeMaterial`) "AlarmState" 0.0)
        (`MaterialInstanceDynamic.SetScalarParameterValue` (`self.LensMaterial`) "AlarmState" 0.0)
        ;[1 0.993 0.095] Determine and transmit Target State to all BP that require notification
        (for _index (range (`KismetArrayLibrary.Array_Length` _bptotriggeralarm)) :!label _label_2
          (message `/Game/BluePrints/TDA_BPs/Interactive_Objects/SecurityCameras/Assets/Blueprints/BPI_Security_Alarm_Interface.Security Alarm Interface` (`|GetArrayItem` _bptotriggeralarm _index) _hastarget)
          ;;[1 1 1] Change Music ?
          (if (`self.MusicChange`)
            (message `/Game/BluePrints/TDA_BPs/Interactive_Objects/SecurityCameras/Assets/Blueprints/BPI_Security_Alarm_Interface.Security Alarm Interface` (`GameplayStatics.GetGameMode`) _hastarget))
          (if _hastarget
            ;[1 1 1] Camera Scan Rotation
            (bind (_direction _scanrotation) (`Timeline|ScanRotationTimeline` :!via `Stop` :!label _label_3)) ; Camera Rotation Anim
            (else
              (goto _label_3 :!via `PlayFromStart`))))))
    (elif (== OtherActor (`GameplayStatics.GetPlayerPawn` 0))
      (set `self.Player` OtherActor)
      (set `self.HasTarget` true) ; Set has target TRUE
      (`GameplayStatics.PlaySoundAtLocation` "/Game/UI/Cardinal/MainMenu/Audio/SoundWaves/TunePeddler/A_Sense_of_Time.A_Sense_of_Time" _returnvalue) ; Lock on Sound
      (`AudioComponent.SetSound` _audioscanner (`self.ScanAlarmCue`)) ; Set Audio to Alarm Loop
      (`ActorComponent.Activate` _audioscanner false) ; Play Audio
      (`LightComponent.SetLightColor` (`self.SpotLight`) (`self.LightColourAlarmOn`) true) ; Alarm ON
      (`MaterialInstanceDynamic.SetScalarParameterValue` (`self.ViewConeMaterial`) "AlarmState" 0.0)
      (`MaterialInstanceDynamic.SetScalarParameterValue` (`self.LensMaterial`) "AlarmState" 0.0)
      (goto _label_2))))

(event `self.ViewCapsule.OnComponentEndOverlap`
  (params (OverlappedComponent :type "PrimitiveComponent Object Reference") (OtherActor :type "Actor Object Reference") (OtherComp :type "PrimitiveComponent Object Reference") (OtherBodyIndex :type Integer))
  ;[1 0.993 0.095] Alarm States and Materials + Light colours
  (if (`self.HasTarget`)
    (goto _label :!via `PlayFromStart`)))

(event `self.ReceiveTick`
  (params (DeltaSeconds :type "Float (single-precision)"))
  (bind _camerapitch (`self.CameraPitch`))
  (bind _cameramaxyaw (`self.CameraMaxYaw`))
  (bind _sm_cctvcamera (`self.SM_CCTVCamera`))
  (bind _pitch (.pitch (`self.DefaultRotation`)))
  (bind _yaw (.yaw (`self.DefaultRotation`)))
  ;[1 1 1] Camera Scan Rotation
  (if (`self.HasTarget`)
    ;[1 0.993 0.095] Tracking Player Pawn
    (`SceneComponent.K2_SetWorldRotation` (`self.SM_CCTVCamera`) (`KismetMathLibrary.MakeRotator` 0.0 (`KismetMathLibrary.ClampAngle` (.pitch (`KismetMathLibrary.MakeRotFromX` (`KismetMathLibrary.VInterpTo` (`KismetMathLibrary.Conv_RotatorToVector` (`SceneComponent.K2_GetComponentRotation` (`self.SM_CCTVCamera`))) (- (`self.K2_GetActorLocation` (`self.Player`)) (`SceneComponent.K2_GetComponentLocation` (`self.SM_CCTVCamera`))) DeltaSeconds 0.01))) (- _pitch 80.0) (+ _pitch 80.0)) (`KismetMathLibrary.ClampAngle` (.yaw (`KismetMathLibrary.MakeRotFromX` (`KismetMathLibrary.VInterpTo` (`KismetMathLibrary.Conv_RotatorToVector` (`SceneComponent.K2_GetComponentRotation` (`self.SM_CCTVCamera`))) (- (`self.K2_GetActorLocation` (`self.Player`)) (`SceneComponent.K2_GetComponentLocation` (`self.SM_CCTVCamera`))) DeltaSeconds 0.01))) (- _yaw 80.0) (+ _yaw 80.0))) false false)
    (else
      (`SceneComponent.K2_SetRelativeRotation` _sm_cctvcamera (`KismetMathLibrary.RInterpTo` (`SceneComponent.RelativeRotation` _sm_cctvcamera) (`KismetMathLibrary.RLerp` (`KismetMathLibrary.MakeRotator` 0.0 _camerapitch _cameramaxyaw) (`KismetMathLibrary.MakeRotator` 0.0 _camerapitch (* _cameramaxyaw -1.0)) (stale `self.SM_Security_Camera_Viewcone.OnComponentBeginOverlap` _scanrotation)) DeltaSeconds 0.3) false false))))

(fn `SceneCaptureActivation`
  (params (Activation :type Boolean))
  (returns (CaptureTexture :type "TextureRenderTarget2D Object Reference"))
  (`SceneComponent.SetVisibility` (`self.SceneCapture`) Activation false)
  (return (`self.SceneCaptureTexture`)))

(fn `UserConstructionScript`
  (bind _scenecapture (`self.SceneCapture`))
  (bind _spotlight (`self.SpotLight`))
  (bind _sm_cctvcamera (`self.SM_CCTVCamera`))
  ;[0.0861 0.5189 0.57] Render to Texture Setup
  (set `SceneCaptureComponent2D.TextureTarget` (`self.SceneCaptureTexture`) _scenecapture)
  (set `SceneCaptureComponent.MaxViewDistanceOverride` (`self.SceneCaptureViewDistance`) _scenecapture)
  ;[0.0861 0.5189 0.57] Spot Light Params
  (`LightComponent.SetIntensity` _spotlight (`self.SpotLightBrightness`))
  (`LightComponent.SetLightColor` _spotlight (`self.LightColourAlarmOff`) true)
  (`PointLightComponent.SetAttenuationRadius` _spotlight (`self.LightAttenuationRadius`))
  ;[0.312 0.3018 0.57] Camera Pitch/YAW Defaults
  (`SceneComponent.K2_SetRelativeRotation` _sm_cctvcamera (`KismetMathLibrary.MakeRotator` 0.0 (`self.CameraPitch`)) false false)
  (set `self.DefaultRotation` (`SceneComponent.K2_GetComponentRotation` _sm_cctvcamera))
  ;[0.312 0.3018 0.57] Camera/Viewcone Materials
  (bind _returnvalue (`PrimitiveComponent.CreateDynamicMaterialInstance` (`self.SM_Security_Camera_Viewcone`) 0 null))
  (set `self.ViewConeMaterial` _returnvalue)
  (bind _returnvalue_2 (`PrimitiveComponent.CreateDynamicMaterialInstance` (`self.SM_CCTVCamera`) 0 null))
  (set `self.LensMaterial` _returnvalue_2))