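; BP_BayDoors is a double sliding bay door actor that opens when something enters its trigger and closes when it leaves.
; On BeginPlay it stores each panel's world location and computes open targets offset in opposite world X and Y directions.
; Overlap begin plays a timeline that lerps both panels between these points, and overlap end reverses it, with no filter on the overlapping actor.
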(event `self.ReceiveBeginPlay`
  (bind _returnvalue (`SceneComponent.K2_GetComponentLocation` (`self.BayDoors_SM_Door2`)))
  (bind _returnvalue_2 (`SceneComponent.K2_GetComponentLocation` (`self.BayDoors_SM_Door`)))
  (set `self.DoorStart` _returnvalue_2)
  (set `self.DoorStart2` _returnvalue)
  (set `self.DoorEnd` (`KismetMathLibrary.MakeVector` (- (.x _returnvalue_2) (`self.OffsetX`)) (- (.y _returnvalue_2) (`self.Offset`)) (.z _returnvalue_2)))
  (set `self.DoorEnd2` (`KismetMathLibrary.MakeVector` (+ (.x _returnvalue) (`self.OffsetX`)) (+ (`self.Offset`) (.y _returnvalue)) (.z _returnvalue))))

(event `self.DoorTrigger.OnComponentBeginOverlap`
  (params (OverlappedComponent :type "PrimitiveComponent Object Reference") (OtherActor :type "Actor Object Reference") (OtherComp :type "PrimitiveComponent Object Reference") (OtherBodyIndex :type Integer) (bFromSweep :type Boolean) (SweepResult :type "HitResult Structure (by ref)"))
  (bind (_direction _newtrack_0) (`Timeline|Timeline_0` :!label _label)
    (:`Update`
      (`SceneComponent.K2_SetWorldLocation` (`self.BayDoors_SM_Door`) (`KismetMathLibrary.VLerp` (`self.DoorStart`) (`self.DoorEnd`) _newtrack_0) false false)
      (`SceneComponent.K2_SetWorldLocation` (`self.BayDoors_SM_Door2`) (`KismetMathLibrary.VLerp` (`self.DoorStart2`) (`self.DoorEnd2`) _newtrack_0) false false))))

(event `self.DoorTrigger.OnComponentEndOverlap`
  (params (OverlappedComponent :type "PrimitiveComponent Object Reference") (OtherActor :type "Actor Object Reference") (OtherComp :type "PrimitiveComponent Object Reference") (OtherBodyIndex :type Integer))
  (goto _label :!via `Reverse`))

(fn `UserConstructionScript`)