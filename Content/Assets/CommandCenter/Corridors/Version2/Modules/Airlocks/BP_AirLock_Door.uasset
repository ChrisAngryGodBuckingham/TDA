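; Airlock door for the command center corridors that slides vertically when the player character enters its trigger volume.
; BeginPlay caches the door's world location as the start and adds a Z offset for the end position.
; Trigger overlap plays a timeline that lerps the door between the two points.
; Leaving the trigger reverses the timeline after a short delay.
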(event `self.ReceiveBeginPlay`
  (bind _returnvalue (`SceneComponent.K2_GetComponentLocation` (`self.AirLockDoor`)))
  (set `self.DoorStart` _returnvalue)
  (set `self.DoorEnd` (`KismetMathLibrary.MakeVector` (.x _returnvalue) (.y _returnvalue) (+ (.z _returnvalue) (`self.OffSetZ`)))))

(event `self.Trigger.OnComponentBeginOverlap`
  (params (OverlappedComponent :type "PrimitiveComponent Object Reference") (OtherActor :type "Actor Object Reference") (OtherComp :type "PrimitiveComponent Object Reference") (OtherBodyIndex :type Integer) (bFromSweep :type Boolean) (SweepResult :type "HitResult Structure (by ref)"))
  (if (== OtherActor (`GameplayStatics.GetPlayerCharacter` 0))
    (bind (_direction _airlockmovement) (`Timeline|AirlockAnim` :!label _label)
      (:`Update`
        (`SceneComponent.K2_SetWorldLocation` (`self.AirLockDoor`) (`KismetMathLibrary.VLerp` (`self.DoorStart`) (`self.DoorEnd`) _airlockmovement) false false)))))

(event `self.Trigger.OnComponentEndOverlap`
  (params (OverlappedComponent :type "PrimitiveComponent Object Reference") (OtherActor :type "Actor Object Reference") (OtherComp :type "PrimitiveComponent Object Reference") (OtherBodyIndex :type Integer))
  (if (== OtherActor (`GameplayStatics.GetPlayerCharacter` 0))
    (`KismetSystemLibrary.Delay` 1.5)
    (goto _label :!via `Reverse`)))

(fn `UserConstructionScript`)